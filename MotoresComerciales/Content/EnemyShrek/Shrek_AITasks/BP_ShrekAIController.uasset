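; AI controller for the Shrek enemy that feeds perceived targets into its follow behavior.
; On BeginPlay it runs the BT_ShrekFollow behavior tree and caches the Blackboard.
; AI Perception updates write any successfully sensed actor to the TargetActor key, with no filtering by actor or sense.
; A failed stimulus clears that key, whichever actor it came from.
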(event OnTargetPerceptionUpdated(AIPerception)
  (params (Actor :type Actor%20Object%20Reference) (Stimulus :type AI%20Stimulus%20Structure))
  (bind _bb (Variables|Default|GetBB))
  (if (.bSuccessfullySensed (Utilities|Struct|BreakAIStimulus Stimulus))
    (AI|Components|Blackboard|SetValueasObject _bb (Utilities|Name|MakeLiteralName "TargetActor") Actor)
    (else
      (AI|Components|Blackboard|ClearValue _bb (Utilities|Name|MakeLiteralName "TargetActor")))))

(event EventBeginPlay
  (AI|RunBehaviorTree "/Game/EnemyShrek/Shrek_AITasks/BT_ShrekFollow.BT_ShrekFollow")
  (Variables|Default|SetBB (AI|GetBlackboard 0)))

(fn ConstructionScript)