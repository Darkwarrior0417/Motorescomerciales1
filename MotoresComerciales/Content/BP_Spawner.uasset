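; BP_Spawner repeatedly spawns waves of BP_NPCE actors around its own location.
; A looping timer started on BeginPlay fires SpawnEnemy every two seconds, with each wave's size derived from NPCAmount.
; Each spawn adds a fixed diagonal offset and a yaw-rotated, unscaled forward vector, so the actors land almost on one point, facing the spawner's rotation.
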(event Custom|Spawn%20Enemy
  (bind _returnvalue (Transformation|GetActorRotation))
  (for _index (range 0 (+ (Variables|Default|GetNPCAmount) 1))
    (Game|SpawnActorfromClass "/Game/ThirdPerson/Blueprints/BP_NPCE.BP_NPCE_C" (Math|Transform|MakeTransform (+ (Transformation|GetActorLocation) (+ (Math|Vector|GetForwardVector (Math|Rotator|CombineRotators _returnvalue (Math|Rotator|MakeRotator 0.0 0.0 (Math|Conversions|ToFloat(Integer) (+ _index (+ 300 (Variables|Default|GetNPCAmount))))))) "100.000000,100.000000,100.000000")) _returnvalue "1.000000,1.000000,1.000000") "Undefined" "MultiplyWithRoot" 0 0)))

(event EventBeginPlay
  (Utilities|Time|SetTimerbyEvent (delegate Custom|Spawn%20Enemy) 2.0 true))

(fn ConstructionScript)