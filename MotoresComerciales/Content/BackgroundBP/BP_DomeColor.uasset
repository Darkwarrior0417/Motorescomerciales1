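; BP_DomeColor is an actor that changes the tint of a sky dome mesh from keyboard input.
; On BeginPlay it switches the player to game-only input and hides the mouse cursor.
; E creates a new dynamic instance of M_Skysphere on DomeMesh and sets its Tint to a fixed mint green.
; R sets Tint back to ColorOriginal on that instance, so it relies on E having run first.
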(event Collision|EventActorBeginOverlap
  (params (OtherActor :type Actor%20Object%20Reference)))

(event EventBeginPlay
  (bind _returnvalue (Game|GetPlayerController 0))
  (Input|SetInputModeGameOnly _returnvalue false)
  (Variables|/Script/Engine.PlayerController|SetbShowMouseCursor _returnvalue false))

(event Input|KeyboardEvents|E
  (params (Key :type Key%20Structure :default "None"))
  (bind _domemesh (Variables|Default|GetDomeMesh))
  (:Pressed
    (bind _returnvalue (Rendering|Material|CreateDynamicMaterialInstance _domemesh 0 "/Game/Textures/HDRI/M_Skysphere.M_Skysphere" "None" :!class /Script/Engine.PrimitiveComponent))
    (Variables|Default|SetDynamicMaterial _returnvalue)
    (Rendering|Material|SetMaterial _domemesh 0 (Variables|Default|GetDynamicMaterial))
    (Rendering|Material|SetVectorParameterValue (Variables|Default|GetDynamicMaterial) "Tint" "(R=0.234761,G=1.000000,B=0.727118,A=1.000000)" :!class /Script/Engine.MaterialInstanceDynamic)))

(event Input|KeyboardEvents|R
  (params (Key :type Key%20Structure :default "None"))
  (:Pressed
    (Rendering|Material|SetVectorParameterValue (Variables|Default|GetDynamicMaterial) "Tint" (Variables|Default|GetColorOriginal) :!class /Script/Engine.MaterialInstanceDynamic)))

(fn ConstructionScript)